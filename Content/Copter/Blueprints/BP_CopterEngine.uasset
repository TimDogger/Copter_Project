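; A single motor and propeller unit of a physics-driven copter, attached to a parent BP_Copter.
; Initialize applies the model's motor mesh and mass, then picks a CW or CCW prop from the roll and pitch ratio signs.
; SetThrottle maps throttle piecewise around a midpoint to motor current.
; While powered and undamaged, Tick converts current through a thrust curve into force and yaw-scaled torque on the copter body, and spins the prop.
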(event `self.ReceiveTick`
  (params (DeltaSeconds :type "Float (single-precision)"))
  (if (`Copter.IsPowerOn` (`self.Copter`))
    (`self.ApplyForce`)))

(fn `ApplyForce`
  (locals (Local_Force :type "Vector Structure" :default (0.0 0.0 0.0)))
  (bind (_ratio_roll _ratio_pitch _ratio_yaw) (break `CopterMotorRatio` (`self.Ratio`)))
  (bind _copter (`self.Copter`))
  (bind (_ratio_roll_2 _ratio_pitch_2 _ratio_yaw_2) (break `CopterMotorRatio` (`self.Ratio`)))
  (bind _returnvalue (`SceneComponent.GetAttachSocketName` (`self.MotorMesh`)))
  (bind (_model_modelname _model_voltage _model_kv _model_noloadcurrent _model_resistance _model_maxcontiniouscurrent _model_maxcontiniouspower _model_mass _model_thrustcurve) (break `/Game/Copter/Structs/Engine_Model2` (`/Game/Copter/Blueprints/BP_Copter.Model` (`self.Copter`))))
  (bind (_model_modelname_2 _model_voltage_2 _model_kv_2 _model_noloadcurrent_2 _model_resistance_2 _model_maxcontiniouscurrent_2 _model_maxcontiniouspower_2 _model_mass_2 _model_thrustcurve_2) (break `/Game/Copter/Structs/Engine_Model2` (`/Game/Copter/Blueprints/BP_Copter.Model` _copter)))
  (bind _returnvalue_2 (`SkinnedMeshComponent.GetSocketBoneName` (`Copter.Mesh` (`self.Copter`)) _returnvalue))
  (bind _returnvalue_location (`KismetMathLibrary.BreakTransform` (`SceneComponent.GetSocketTransform` (`Copter.Mesh` (`self.Copter`)) _returnvalue "RTS_World")))
  (if (`self.IsNotDamaged`)
    (bind _output_get (set `local.Local_Force` (* (`SceneComponent.GetUpVector` (`self.MotorMesh`)) (`CurveFloat.GetFloatValue` _model_thrustcurve (`self.Current`)))))
    (`PrimitiveComponent.AddForceAtLocation` (`Copter.Mesh` (`self.Copter`)) _output_get _returnvalue_location _returnvalue_2)
    (`PrimitiveComponent.AddTorqueInRadians` (`Copter.Mesh` (`self.Copter`)) (* (`local.Local_Force`) _ratio_yaw_2) _returnvalue_2 false)
    (`SceneComponent.K2_AddRelativeRotation` (`self.PropMesh`) (`KismetMathLibrary.MakeRotator` 0.0 0.0 (* (`KismetMathLibrary.MapRangeClamped` (`CurveFloat.GetFloatValue` _model_thrustcurve_2 (`self.Current`)) (`Copter.EngineMinCurrent` _copter) (`Copter.EngineMaxCurrent` _copter) 10.0 30.0) _ratio_yaw)) false false)))

(fn `Initialize`
  (params (Ratio :type "CopterMotorRatio Structure"))
  (locals (Local_ThrustCurve :type "CurveFloat Object Reference") (Local_PropMesh :type "StaticMesh Object Reference") (Local_Model :type "/Game/Copter/Structs/Engine_Model2 Structure"))
  (bind (_local_model_modelname _local_model_voltage _local_model_kv _local_model_noloadcurrent _local_model_resistance _local_model_maxcontiniouscurrent _local_model_maxcontiniouspower _local_model_mass _local_model_thrustcurve) (break `/Game/Copter/Structs/Engine_Model2` (`local.Local_Model`)))
  (bind _copter (`self.Copter`))
  (bind (_local_model_modelname_2 _local_model_voltage_2 _local_model_kv_2 _local_model_noloadcurrent_2 _local_model_resistance_2 _local_model_maxcontiniouscurrent_2 _local_model_maxcontiniouspower_2 _local_model_mass_2 _local_model_thrustcurve_2 _local_model_mesh) (break `/Game/Copter/Structs/Engine_Model2` (`local.Local_Model`)))
  (bind (_ratio_roll _ratio_pitch) (break `CopterMotorRatio` (`self.Ratio`)))
  (bind _propmesh (`self.PropMesh`))
  (bind _mesh (`Copter.Mesh` (`self.Copter`)))
  (set `self.Ratio` Ratio)
  (if (not (>= (`KismetStringLibrary.Len` (`KismetStringLibrary.Conv_NameToString` (`self.EngineSocket`))) 0))
    (set `self.EngineSocket` (`self.GetAttachParentSocketName`)))
  (bind _asbp_copter (cast `/Game/Copter/Blueprints/BP_Copter` (`self.GetAttachParentActor`))
    (:`then`
      (set `self.Copter` _asbp_copter)
      (set `local.Local_Model` (`/Game/Copter/Blueprints/BP_Copter.Model` (`self.Copter`)))
      (set `local.Local_ThrustCurve` _local_model_thrustcurve)
      (`|ExecutionSequence`
        (:`then_0`
          ;[1 1 1] Comment
          (`StaticMeshComponent.SetStaticMesh` (`self.MotorMesh`) _local_model_mesh)
          (`PrimitiveComponent.SetSimulatePhysics` (`self.MotorMesh`) false)
          (`PrimitiveComponent.SetMassOverrideInKg` _mesh (`SkinnedMeshComponent.GetSocketBoneName` _mesh (`SceneComponent.GetAttachSocketName` (`self.MotorMesh`))) _local_model_mass_2 true)
          (set `/Game/Copter/Blueprints/BP_Copter.CopterMass` (`PrimitiveComponent.GetMass` (`Copter.Mesh` _copter)) _copter))
        (:`then_1`
          (if (> (* _ratio_roll _ratio_pitch) 0.0)
            (set `local.Local_PropMesh` "/Game/Copter/Meshes/MiDrone/Xiaomi_Mi_Drone_Motor_Prop_CCW.Xiaomi_Mi_Drone_Motor_Prop_CCW")
            (else
              (set `local.Local_PropMesh` "/Game/Copter/Meshes/MiDrone/Xiaomi_Mi_Drone_Motor_Prop_CW.Xiaomi_Mi_Drone_Motor_Prop_CW")))
          (`StaticMeshComponent.SetStaticMesh` _propmesh (`local.Local_PropMesh`))
          (`PrimitiveComponent.SetSimulatePhysics` _propmesh false)
          (`PrimitiveComponent.SetMassOverrideInKg` (`self.PropMesh`) "None" 0.1 true)
          (if (`KismetArrayLibrary.Array_Contains` (`SceneComponent.GetAllSocketNames` (`self.MotorMesh`)) (`self.SocketName_Prop`))
            (`SceneComponent.K2_SetRelativeTransform` (`self.PropMesh`) (`SceneComponent.GetSocketTransform` (`self.MotorMesh`) (`self.SocketName_Prop`) "RTS_Actor") false false)
            (else
              (`KismetSystemLibrary.PrintString` (`KismetStringLibrary.Concat_StrStr` (`KismetSystemLibrary.GetObjectName` self) " Does Not Have Prop Socket Named: " (`KismetStringLibrary.Conv_NameToString` (`self.SocketName_Prop`))) true true (struct :`G` 0.66 :`B` 1.0 :`A` 1.0) 10.0))))))
    (:`CastFailed`
      (`KismetSystemLibrary.PrintString` "Parent class not a Copter"))))

(fn `SetThrottle`
  (params (Throttle :type "Float (double-precision)"))
  (returns (Value :type "Float (double-precision)"))
  (bind _copter (`self.Copter`))
  (bind _copter_2 (`self.Copter`))
  (bind _output_get (set `self.Throttle` Throttle))
  (`self.CompareFloatWithTolerance` _output_get 50.0 0.1
    (:`>`
      (set `self.Current` (`KismetMathLibrary.MapRangeClamped` (`self.Throttle`) 50.0 100.0 (`Copter.EngineMidCurrent` _copter_2) (`Copter.EngineMaxCurrent` _copter_2))))
    (:`=`
      (set `self.Current` (`Copter.EngineMidCurrent` (`self.Copter`))))
    (:`<`
      (set `self.Current` (`KismetMathLibrary.MapRangeClamped` (`self.Throttle`) 0.0 50.0 (`Copter.EngineMinCurrent` _copter) (`Copter.EngineMidCurrent` _copter)))))
  (return (`self.Throttle`)))

(fn `UserConstructionScript`)