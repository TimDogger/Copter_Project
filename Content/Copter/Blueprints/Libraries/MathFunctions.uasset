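; Math function library in the Copter project that does reverse lookups on float curves, finding the input whose curve value matches a target.
; Both functions run a golden-section search between Left and Right, narrowing the bracket by the absolute error at two probe points for up to 501 iterations.
; One uses a fixed tolerance, the other takes it as a parameter.
; The result is only assigned when a probe lands within tolerance.
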(fn `GetValueByCurveFloat`
  (params (Target :type "Float (double-precision)") (Left :type "Float (double-precision)") (Right :type "Float (double-precision)") (Curve :type "CurveFloat Object Reference"))
  (returns (Result :type "Float (double-precision)"))
  (locals (Local_TargetValue :type "Float (double-precision)") (Local_Tolerance :type "Float (double-precision)" :default 0.0001) (Local_A :type "Float (double-precision)") (Local_B :type "Float (double-precision)") (Local_X1 :type "Float (double-precision)") (Local_X2 :type "Float (double-precision)") (Local_Curve :type "CurveFloat Object Reference") (Local_X1_Value :type "Float (double-precision)") (Local_X2_Value :type "Float (double-precision)") (Local_Result :type "Float (double-precision)"))
  (bind _local_curve (`local.Local_Curve`))
  (set `local.Local_A` Left)
  (set `local.Local_B` Right)
  (set `local.Local_TargetValue` Target)
  (set `local.Local_Curve` Curve)
  (for _ (range 501)
    (set `local.Local_X1` (- (`local.Local_B`) (/ (- (`local.Local_B`) (`local.Local_A`)) 1.618)))
    (set `local.Local_X2` (+ (`local.Local_A`) (/ (- (`local.Local_B`) (`local.Local_A`)) 1.618)))
    (set `local.Local_X1_Value` (`CurveFloat.GetFloatValue` _local_curve (`local.Local_X1`)))
    (set `local.Local_X2_Value` (`CurveFloat.GetFloatValue` _local_curve (`local.Local_X2`)))
    (if (>= (`KismetMathLibrary.Abs` (- (`local.Local_TargetValue`) (`local.Local_X1_Value`))) (`KismetMathLibrary.Abs` (- (`local.Local_TargetValue`) (`local.Local_X2_Value`))))
      (set `local.Local_A` (`local.Local_X1`))
      (if (`KismetMathLibrary.NearlyEqual_FloatFloat` (`local.Local_X1_Value`) (`local.Local_TargetValue`) 0.001)
        (set `local.Local_Result` (`local.Local_X1`))
        (break))
      (else
        (set `local.Local_B` (`local.Local_X2`))
        (if (`KismetMathLibrary.NearlyEqual_FloatFloat` (`local.Local_X2_Value`) (`local.Local_TargetValue`) 0.001)
          (set `local.Local_Result` (`local.Local_X2`))
          (break)))))
  (return (`local.Local_Result`)))

(fn `GetValueByCurveFloatWithTolerance`
  (params (Target :type "Float (double-precision)") (Left :type "Float (double-precision)") (Right :type "Float (double-precision)") (NewParam :type "Float (double-precision)") (Curve :type "CurveFloat Object Reference"))
  (returns (Result :type "Float (double-precision)"))
  (locals (Local_TargetValue :type "Float (double-precision)") (Local_Tolerance :type "Float (double-precision)" :default 0.0001) (Local_A :type "Float (double-precision)") (Local_B :type "Float (double-precision)") (Local_X1 :type "Float (double-precision)") (Local_X2 :type "Float (double-precision)") (Local_Curve :type "CurveFloat Object Reference") (Local_X1_Value :type "Float (double-precision)") (Local_X2_Value :type "Float (double-precision)") (Local_Result :type "Float (double-precision)"))
  (bind _local_curve (`local.Local_Curve`))
  (set `local.Local_A` Left)
  (set `local.Local_B` Right)
  (set `local.Local_TargetValue` Target)
  (set `local.Local_Tolerance` NewParam)
  (set `local.Local_Curve` Curve)
  (for _ (range 501)
    (set `local.Local_X1` (- (`local.Local_B`) (/ (- (`local.Local_B`) (`local.Local_A`)) 1.618)))
    (set `local.Local_X2` (+ (`local.Local_A`) (/ (- (`local.Local_B`) (`local.Local_A`)) 1.618)))
    (set `local.Local_X1_Value` (`CurveFloat.GetFloatValue` _local_curve (`local.Local_X1`)))
    (set `local.Local_X2_Value` (`CurveFloat.GetFloatValue` _local_curve (`local.Local_X2`)))
    (if (>= (`KismetMathLibrary.Abs` (- (`local.Local_TargetValue`) (`local.Local_X1_Value`))) (`KismetMathLibrary.Abs` (- (`local.Local_TargetValue`) (`local.Local_X2_Value`))))
      (set `local.Local_A` (`local.Local_X1`))
      (if (`KismetMathLibrary.NearlyEqual_FloatFloat` (`local.Local_X1_Value`) (`local.Local_TargetValue`) (`local.Local_Tolerance`))
        (set `local.Local_Result` (`local.Local_X1`))
        (break))
      (else
        (set `local.Local_B` (`local.Local_X2`))
        (if (`KismetMathLibrary.NearlyEqual_FloatFloat` (`local.Local_X2_Value`) (`local.Local_TargetValue`) (`local.Local_Tolerance`))
          (set `local.Local_Result` (`local.Local_X2`))
          (break)))))
  (return (`local.Local_Result`)))