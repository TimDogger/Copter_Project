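; PID1 is a copter library with a single GetValue function that computes a PID controller output from an error and time step.
; It sums proportional, integral and derivative terms using PID gains, taking the derivative from the change since the caller-supplied previous error.
; It returns the force and current error for the next call.
; The error sum is function-local, so the integral term sees only the current error and does not accumulate across calls.
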(fn `GetValue`
  (params (PrevError :type "Float (double-precision)") (Delta :type "Float (double-precision)") (DeltaTime :type "Float (double-precision)") (PID :type "/Game/Copter/Structs/K_PID Structure (by ref)"))
  (returns (PrevDeltaOut :type "Float (double-precision)") (Value :type "Float (double-precision)"))
  (locals (Local_PrevError :type "Float (double-precision)") (Local_Delta :type "Float (double-precision)") (Local_ErrorSum :type "Float (double-precision)") (Local_Force :type "Float (double-precision)") (Local_DeltaTime :type "Float (double-precision)"))
  (bind (_p _i _d) (break `/Game/Copter/Structs/K_PID` PID))
  (set `local.Local_PrevError` PrevError)
  (set `local.Local_Delta` Delta)
  (set `local.Local_DeltaTime` DeltaTime)
  (set `local.Local_ErrorSum` (+ (`local.Local_Delta`) (`local.Local_ErrorSum`)))
  (set `local.Local_Force` (+ (* (`local.Local_Delta`) _p) (* (`local.Local_ErrorSum`) _i (`local.Local_DeltaTime`)) (/ (* _d (- (`local.Local_Delta`) (`local.Local_PrevError`))) (`local.Local_DeltaTime`))))
  (return (`local.Local_Delta`) (`local.Local_Force`)))