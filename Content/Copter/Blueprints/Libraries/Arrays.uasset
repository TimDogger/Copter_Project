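; Blueprint function library of array helpers for strings and names.
; FindStringInArray returns the index of the first matching string, branching on a case-sensitivity flag.
; FilterArray uses it to gather numbered entries (FilterName_0, FilterName_1 and so on) in order, stopping at the first missing number.
; Two converters turn Name arrays into String arrays and back, element by element.
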(fn `ConvertArrayNameToString`
  (params (Array :type "Array of Name"))
  (returns (Result :type "Array of String"))
  (locals (Local_Array :type "Array of String"))
  (for (_array_element _array_index) Array
    (`KismetArrayLibrary.Array_Set` (`local.Local_Array`) _array_index (`KismetStringLibrary.Conv_NameToString` _array_element) true))
  (return (`local.Local_Array`)))

(fn `ConvertArrayStringToName`
  (params (Array :type "Array of String"))
  (returns (Result :type "Array of Name"))
  (locals (Local_Array :type "Array of Name"))
  (for (_array_element _array_index) Array
    (`KismetArrayLibrary.Array_Set` (`local.Local_Array`) _array_index (`KismetStringLibrary.Conv_StringToName` _array_element) true))
  (return (`local.Local_Array`)))

(fn `FilterArray`
  (params (FilterName :type String) (Source :type "Array of String"))
  (returns (FilteredArray :type "Array of String"))
  (locals (Local_FilterName :type String) (Local_SourceArray :type "Array of String") (Local_StillSearching :type Boolean) (Local_SearchName :type String) (Local_TargetArray :type "Array of String"))
  (bind _indexofstring (`self.FindStringInArray` (`local.Local_SearchName`) (`local.Local_SourceArray`)))
  (set `local.Local_FilterName` FilterName)
  (set `local.Local_SourceArray` Source)
  (set `local.Local_StillSearching` true)
  (while (`local.Local_StillSearching`)
    (set `local.Local_SearchName` (`KismetStringLibrary.Concat_StrStr` (`local.Local_FilterName`) "_" (`KismetStringLibrary.Conv_IntToString` (`KismetArrayLibrary.Array_Length` (`local.Local_TargetArray`)))))
    (if (!= _indexofstring -1)
      (`KismetArrayLibrary.Array_Add` (`local.Local_TargetArray`) (`|GetArrayItem` (`local.Local_SourceArray`) _indexofstring))
      (else
        (set `local.Local_StillSearching` false))))
  (return (`local.Local_TargetArray`)))

(fn `FindStringInArray`
  (params (StringToFind :type String) (SourceArray :type "Array of String") (CaseSensetive :type Boolean))
  (returns (IndexOfString :type Integer))
  (locals (Local_StringToFind :type String) (Local_SourceArray :type "Array of String") (Local_Index :type Integer :default -1))
  (set `local.Local_StringToFind` StringToFind)
  (set `local.Local_SourceArray` SourceArray)
  (if CaseSensetive
    (for (_array_element _array_index) (`local.Local_SourceArray`)
      (if (`KismetStringLibrary.EqualEqual_StrStr` _array_element (`local.Local_StringToFind`))
        (set `local.Local_Index` _array_index)
        (break)))
    (else
      (for (_array_element_2 _array_index_2) (`local.Local_SourceArray`)
        (if (== _array_element_2 (`local.Local_StringToFind`))
          (set `local.Local_Index` _array_index_2)
          (break)))))
  (return (`local.Local_Index`)))