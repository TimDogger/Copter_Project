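; BP_Operator is an operator actor that broadcasts a message to the BP_Copter actors within range of its Sphere component.
; UpdateCopters rebuilds the Copters list from sphere overlaps, keeping only those whose actor distance is within the sphere radius.
; SendMessage refreshes that list and calls Receive on each copter whose LastMessage differs, passing the whole list as CoptersToIgnore.
; The event graph holds no active logic.
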(fn `SendMessage`
  (params (Message :type String))
  (bind _copters (`self.UpdateCopters`))
  (for _array_element _copters
    (if (`KismetStringLibrary.NotEqual_StrStr` (`/Game/Copter/Blueprints/BP_Copter.LastMessage` _array_element) Message)
      (`/Game/Copter/Blueprints/BP_Copter.Receive` _array_element Message (`self.Copters`)))))

(fn `UpdateCopters`
  (returns (Copters :type "Array of /Game/Copter/Blueprints/BP_Copter Object Reference"))
  (locals (Local_Copters :type "Array of /Game/Copter/Blueprints/BP_Copter Object Reference"))
  (`KismetArrayLibrary.Array_Clear` (`self.Copters`))
  (for _array_element (`PrimitiveComponent.GetOverlappingActors` (`self.Sphere`) "/Game/Copter/Blueprints/BP_Copter.BP_Copter_C")
    (bind _asbp_copter (cast `/Game/Copter/Blueprints/BP_Copter` _array_element))
    (if (<= (`self.GetDistanceTo` _asbp_copter) (`SphereComponent.SphereRadius` (`self.Sphere`)))
      (`KismetArrayLibrary.Array_Add` (`self.Copters`) _asbp_copter)))
  (return (`self.Copters`)))

(fn `UserConstructionScript`)