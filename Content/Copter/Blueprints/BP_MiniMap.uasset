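; Minimap camera actor for the copter game, offering panning, smoothed spring-arm zoom and drag-box selection of actors.
; Pan speed scales with zoom distance.
; While selecting, Tick rebuilds a collision-enabled procedural pyramid from the camera through the dragged rectangle, flipping triangle winding by drag direction.
; Mouse traces come from the CopterController's minimap widget, which receives the pyramid's overlapping actors as its selection.
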(event `self.ReceiveTick`
  (params (DeltaSeconds :type "Float (single-precision)"))
  (set `self.Delta` DeltaSeconds)
  (set `SpringArmComponent.TargetArmLength` (`KismetMathLibrary.FInterpTo` (`SpringArmComponent.TargetArmLength` (`self.SpringArm`)) (`self.TargetArmLength`) (`self.Delta`) 10.0) (`self.SpringArm`))
  (`self.UpdateSelectionPyramid`))

(event `self.ReceiveBeginPlay`
  (bind _ascopter_controller (cast `/Game/Copter/Blueprints/CopterController` (`GameplayStatics.GetPlayerController` 0))
    (:`then`
      (set `self.ControllerRef` _ascopter_controller)
      (set `self.TargetArmLength` (`SpringArmComponent.TargetArmLength` (`self.SpringArm`))))
    (:`CastFailed`
      (`KismetSystemLibrary.PrintString` "Minimap: Cast To Copter Controller Error" true true (struct :`G` 0.66 :`B` 1.0 :`A` 1.0) 5.0))))

(fn `MoveX`
  (params (X :type "Float (double-precision)"))
  (if (`self.IsMoveable`)
    (`self.K2_AddActorLocalOffset` self (`KismetMathLibrary.MakeVector` 0.0 (* X (`self.ViewMiltipler`) -1.0)) false false)))

(fn `MoveY`
  (params (Y :type "Float (double-precision)"))
  (if (`self.IsMoveable`)
    (`self.K2_AddActorLocalOffset` self (`KismetMathLibrary.MakeVector` (* Y (`self.ViewMiltipler`) -1.0)) false false)))

(fn `StartSelecting`
  (params (StartSelectingLocation :type "Vector Structure"))
  (set `self.StartSelectingLocation` StartSelectingLocation)
  (set `self.IsSelecting` true)
  (`BlueprintMapLibrary.Map_Clear` (`self.OverlappedAndSelectedActors`)))

(fn `StopSelecting`
  (set `self.IsSelecting` false)
  (`ProceduralMeshComponent.ClearAllMeshSections` (`self.Selector`)))

(fn `UpdateSelectionBox`
  (locals (Local_StartPosition :type "Vector Structure") (Local_EndPosition :type "Vector Structure"))
  (bind (_locationx _locationy) (`PlayerController.GetMousePosition` (`self.ControllerRef`)))
  (bind _returnvalue (`SceneComponent.K2_GetComponentLocation` (`self.Scene`)))
  (if (`self.IsSelecting`)
    (set `self.StopSelectingLocation` (`/Game/Copter/Blueprints/Widgets/W_Minimap.LineTraceFromViewport` (`/Game/Copter/Blueprints/CopterController.MinimapWidget` (`self.ControllerRef`)) (`KismetMathLibrary.MakeVector2D` _locationx _locationy)))
    (set `local.Local_StartPosition` (- (`self.StartSelectingLocation`) _returnvalue))
    (set `local.Local_EndPosition` (- (`self.StopSelectingLocation`) _returnvalue))))

(fn `UpdateSelectionPyramid`
  (locals (Local_StartPosition :type "Vector Structure") (Local_EndPosition :type "Vector Structure") (Local_ClassFilter :type "Actor Class Reference") (Local_Triangles :type "Array of Integer") (Vertice1 :type "Vector Structure") (Vertice2 :type "Vector Structure") (Vertice3 :type "Vector Structure") (Vertice4 :type "Vector Structure") (Local_Z :type "Float (double-precision)") (Local_OverlappedActor :type "Actor Object Reference"))
  (bind _local_z (`local.Local_Z`))
  (bind (_local_endposition_x _local_endposition_y) (`KismetMathLibrary.BreakVector` (`local.Local_EndPosition`)))
  (bind _local_startposition_x (`KismetMathLibrary.BreakVector` (`local.Local_StartPosition`)))
  (bind _local_endposition_x_2 (`KismetMathLibrary.BreakVector` (`local.Local_EndPosition`)))
  (bind (_local_startposition_x_2 _local_startposition_y) (`KismetMathLibrary.BreakVector` (`local.Local_StartPosition`)))
  (bind (_startselectinglocation_x _startselectinglocation_y _startselectinglocation_z) (`KismetMathLibrary.BreakVector` (`self.StartSelectingLocation`)))
  (bind (_stopselectinglocation_x _stopselectinglocation_y _stopselectinglocation_z) (`KismetMathLibrary.BreakVector` (`self.StopSelectingLocation`)))
  (bind (_returnvalue_x _returnvalue_y) (`KismetMathLibrary.BreakVector` (- (`local.Local_StartPosition`) (`local.Local_EndPosition`))))
  (bind (_locationx _locationy) (`PlayerController.GetMousePosition` (`self.ControllerRef`)))
  (bind _returnvalue (`SceneComponent.K2_GetComponentLocation` (`self.Scene`)))
  (bind _array (`|MakeArray` (- (`SceneComponent.K2_GetComponentLocation` (`self.Camera`)) (`SceneComponent.K2_GetComponentLocation` (`self.Scene`))) (`local.Vertice1`) (`local.Vertice2`) (`local.Vertice3`) (`local.Vertice4`)))
  (if (`self.IsSelecting`)
    (`|ExecutionSequence`
      (:`then_0`
        (set `self.StopSelectingLocation` (`/Game/Copter/Blueprints/Widgets/W_Minimap.LineTraceFromViewport` (`/Game/Copter/Blueprints/CopterController.MinimapWidget` (`self.ControllerRef`)) (`KismetMathLibrary.MakeVector2D` _locationx _locationy)))
        (set `local.Local_StartPosition` (- (`self.StartSelectingLocation`) _returnvalue))
        (set `local.Local_EndPosition` (- (`self.StopSelectingLocation`) _returnvalue))
        (if (< _startselectinglocation_z _stopselectinglocation_z)
          (set `local.Local_Z` (* _startselectinglocation_z -2.0))
          (else
            (set `local.Local_Z` (* _stopselectinglocation_z -2.0))))
        (set `local.Vertice1` (`KismetMathLibrary.MakeVector` _local_startposition_x_2 _local_startposition_y _local_z))
        (set `local.Vertice2` (`KismetMathLibrary.MakeVector` _local_endposition_x_2 _local_startposition_y _local_z))
        (set `local.Vertice3` (`KismetMathLibrary.MakeVector` _local_startposition_x _local_endposition_y _local_z))
        (set `local.Vertice4` (`KismetMathLibrary.MakeVector` _local_endposition_x _local_endposition_y _local_z))
        (if (> (* _returnvalue_x _returnvalue_y) 0.0)
          (set `local.Local_Triangles` (`|MakeArray` 0 2 1 2 0 4 0 1 3 0 3 4 1 2 3 4 3 2))
          (else
            (set `local.Local_Triangles` (`|MakeArray` 0 1 2 2 4 0 0 3 1 0 4 3 1 3 2 4 2 3))))
        (`ProceduralMeshComponent.CreateMeshSection_LinearColor` :`self` (`self.Selector`) :`Vertices` _array :`Triangles` (`local.Local_Triangles`) :`Normals` _array :`bCreateCollision` true))
      (:`then_1`
        (set `/Game/Copter/Blueprints/Widgets/W_Minimap.SelectedActors` (`PrimitiveComponent.GetOverlappingActors` (`self.Selector`) (`self.ClassFilter`)) (`/Game/Copter/Blueprints/CopterController.MinimapWidget` (`self.ControllerRef`)))))))

(fn `UserConstructionScript`)

(fn `Zoom`
  (params (Axis :type "Float (double-precision)"))
  (bind _output_get (set `self.TargetArmLength` (`KismetMathLibrary.FClamp` (+ (* Axis (`self.ZoomMultipler`) -1.0) (`self.TargetArmLength`)) 500.0 20000.0)))
  (set `self.ViewMiltipler` (/ _output_get 40.0)))