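; Player controller for a copter flight sim, handling flight input, camera switching, engine toggling, position resets and a minimap mode.
; On BeginPlay it caches the BP_Copter pawn, spawns the minimap pawn and creates the debug and minimap widgets.
; Toggling the map swaps possession and HUD, and SwitchPawns routes most inputs by possessed pawn.
; Each tick it refreshes flight telemetry and applies randomly drifting wind force to every copter.
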(event `Key|T`
  (params (Key :type "Key Structure"))
  ;[1 1 1 1 100] HUD
  (:`Pressed`
    (`self.SwitchPawns`
      (:`Copter`
        (set `self.bShowMouseCursor` (not (`self.bShowMouseCursor`)))))))

(event `Key|Escape`
  (params (Key :type "Key Structure"))
  ;[1 1 1 1 100] HUD
  (:`Pressed`
    (`KismetSystemLibrary.QuitGame` null "Quit")))

(event `InputAction|Camera | Switch`
  (params (Key :type "Key Structure"))
  (bind _controlledcopter (`self.ControlledCopter`))
  ;[0 0.1034 1 1 100] Camera
  (:`Pressed`
    (`ActorComponent.ToggleActive` (`/Game/Copter/Blueprints/BP_Copter.CameraFPV` _controlledcopter))
    (`ActorComponent.ToggleActive` (`/Game/Copter/Blueprints/BP_Copter.Camera3PV` _controlledcopter))))

(event `InputAxis|View X`
  (params (AxisValue :type "Float (single-precision)"))
  ;[0 0.1034 1 1 100] Camera
  (`self.SwitchPawns`
    (:`Copter`
      (if (not (`self.bShowMouseCursor`))
        (`/Game/Copter/Blueprints/BP_Copter.AddCameraYaw` (`self.ControlledCopter`) (* (`self.ViewMultiplerX`) AxisValue))))
    (:`Minimap`
      (`/Game/Copter/Blueprints/BP_MiniMap.MoveX` (`self.MiniMap`) AxisValue))))

(event `self.ReceiveTick`
  (params (DeltaSeconds :type "Float (single-precision)"))
  ;[1 1 1 1 100] Main
  (message `/Game/Copter/Interfaces/i_Copter_State.SetRoll` (`self.CopterControllerWidget`) (`Copter.Roll` (`self.ControlledCopter`)))
  (message `/Game/Copter/Interfaces/i_Copter_State.SetPitch` (`self.CopterControllerWidget`) (`Copter.Pitch` (`self.ControlledCopter`)))
  (message `/Game/Copter/Interfaces/i_Copter_State.SetYaw` (`self.CopterControllerWidget`) (`Copter.Yaw` (`self.ControlledCopter`)))
  (message `/Game/Copter/Interfaces/i_Copter_Input.SetTargetRoll` (`self.CopterControllerWidget`) (`Copter.RollSetpoint` (`self.ControlledCopter`)))
  (message `/Game/Copter/Interfaces/i_Copter_Input.SetTargetPitch` (`self.CopterControllerWidget`) (`Copter.PitchSetpoint` (`self.ControlledCopter`)))
  (message `/Game/Copter/Interfaces/i_Copter_Input.SetTargetYaw` (`self.CopterControllerWidget`) (`Copter.YawSetpoint` (`self.ControlledCopter`)))
  (message `/Game/Copter/Interfaces/i_Copter_Throttle.SetThrottle` (`self.CopterControllerWidget`) (`Copter.Throttle` (`self.ControlledCopter`)))
  (message `/Game/Copter/Interfaces/i_Copter_State.SetAltitude` (`self.CopterControllerWidget`) (`Copter.Altitude` (`self.ControlledCopter`)))
  (message `/Game/Copter/Interfaces/i_Copter_State.SetEngines` (`self.CopterControllerWidget`) (`/Game/Copter/Blueprints/BP_Copter.Motors` (`self.ControlledCopter`)))
  (`self.UpdateWind`))

(event `InputAxis|View Y`
  (params (AxisValue :type "Float (single-precision)"))
  ;[0 0.1034 1 1 100] Camera
  (`self.SwitchPawns`
    (:`Copter`
      (if (not (`self.bShowMouseCursor`))
        (`/Game/Copter/Blueprints/BP_Copter.AddCameraPitch` (`self.ControlledCopter`) (* (`self.ViewMultiplerY`) AxisValue))))
    (:`Minimap`
      (`/Game/Copter/Blueprints/BP_MiniMap.MoveY` (`self.MiniMap`) AxisValue))))

(event `self.ReceiveBeginPlay`
  (bind _coptercontrollerwidget (`self.CopterControllerWidget`))
  ;[1 1 1 1 100] Main
  (bind _asbp_copter (cast `/Game/Copter/Blueprints/BP_Copter` (`GameplayStatics.GetPlayerPawn` 0)))
  (set `self.ControlledCopter` _asbp_copter)
  (bind _returnvalue (`|SpawnActorFromClass` "/Game/Copter/Blueprints/BP_MiniMap.BP_MiniMap_C" (`KismetMathLibrary.MakeTransform` (`self.K2_GetActorLocation` (`self.ControlledCopter`))) "Undefined" "OverrideRootScale" null null))
  (set `self.MiniMap` _returnvalue)
  (`|ExecutionSequence`
    (:`then_0`
      (bind _returnvalue_2 (`|CreateWidget` "/Game/Copter/Blueprints/Widgets/W_DebugController.W_DebugController_C" self))
      (set `self.CopterControllerWidget` _returnvalue_2)
      (bind _returnvalue_3 (`|CreateWidget` "/Game/Copter/Blueprints/Widgets/W_Minimap.W_Minimap_C" self))
      (set `self.MinimapWidget` _returnvalue_3))
    (:`then_1`
      (set `/Game/Copter/Blueprints/Widgets/W_Minimap.ControllerRef` self (`self.MinimapWidget`))
      (set `/Game/Copter/Blueprints/Widgets/W_Minimap.MinimapRef` (`self.MiniMap`) (`self.MinimapWidget`))
      (`UserWidget.AddToViewport` (`self.CopterControllerWidget`) 0)
      (`UserWidget.AddToViewport` (`self.MinimapWidget`) 0)
      (`Widget.SetVisibility` (`self.MinimapWidget`) "Collapsed")
      (`Widget.SetVisibility` (`self.CopterControllerWidget`) "Visible"))
    (:`then_2`
      (bind _returnvalue_4 (`GameUserSettings.GetGameUserSettings`))
      (set `self.ScreenResolution` (`GameUserSettings.GetScreenResolution` _returnvalue_4))
      (set `/Game/Copter/Blueprints/Widgets/W_DebugController.Copter` (`self.ControlledCopter`) _coptercontrollerwidget)
      (`/Game/Copter/Blueprints/Widgets/W_DebugController.SetComboPID` _coptercontrollerwidget))))

(event `Key|SpaceBar`
  (params (Key :type "Key Structure"))
  (bind _controlledcopter (`self.ControlledCopter`))
  (:`Pressed`
    (`PrimitiveComponent.SetSimulatePhysics` (`Copter.Mesh` _controlledcopter) false)
    (`Copter.StopFly` _controlledcopter)
    (`self.K2_SetActorLocationAndRotation` :`self` (`self.ControlledCopter`) :`NewLocation` (0.0 0.0 100.0) :`bTeleport` true)
    (`PrimitiveComponent.SetSimulatePhysics` (`Copter.Mesh` (`self.ControlledCopter`)) true)))

(event `InputAxis|Copter | Roll`
  (params (AxisValue :type "Float (single-precision)"))
  ;[0 1 0.3162 1 100] Control
  (`self.SwitchPawns`
    (:`Copter`
      (`Copter.AddCopterRollInput` (`self.ControlledCopter`) AxisValue))))

(event `InputAction|Copter | Toogle Engines`
  (params (Key :type "Key Structure"))
  ;[0 1 0.3162 1 100] Control
  (:`Pressed`
    (if (`Copter.IsPowerOn` (`self.ControlledCopter`))
      (`Copter.StopFly` (`self.ControlledCopter`))
      (else
        (`Copter.StartFly` (`self.ControlledCopter`))))))

(event `InputAction|Map | View`
  (params (Key :type "Key Structure"))
  ;[0.08618 0.3428 1 1 100] Map
  (:`Pressed`
    (set `/Game/Copter/Blueprints/BP_MiniMap.IsMoveable` true (`self.MiniMap`))
    (set `self.bShowMouseCursor` false))
  (:`Released`
    (set `/Game/Copter/Blueprints/BP_MiniMap.IsMoveable` false (`self.MiniMap`))
    (set `self.bShowMouseCursor` true)))

(event `InputAction|Camera | ZoomIn`
  (params (Key :type "Key Structure"))
  ;[0.08618 0.3428 1 1 100] Map
  (:`Pressed`
    (`self.SwitchPawns`
      (:`Minimap`
        (`/Game/Copter/Blueprints/BP_MiniMap.Zoom` (`self.MiniMap`) 1.0)))))

(event `InputAxis|Copter | Pitch`
  (params (AxisValue :type "Float (single-precision)"))
  ;[0 1 0.3162 1 100] Control
  (`self.SwitchPawns`
    (:`Copter`
      (`Copter.AddCopterPitchInput` (`self.ControlledCopter`) AxisValue))))

(event `InputAction|Camera | ZoomOut`
  (params (Key :type "Key Structure"))
  ;[0.08618 0.3428 1 1 100] Map
  (:`Pressed`
    (`self.SwitchPawns`
      (:`Minimap`
        (`/Game/Copter/Blueprints/BP_MiniMap.Zoom` (`self.MiniMap`) -1.0)))))

(event `InputAxis|Copter | Yaw`
  (params (AxisValue :type "Float (single-precision)"))
  ;[0 1 0.3162 1 100] Control
  (`self.SwitchPawns`
    (:`Copter`
      (`Copter.AddCopterYawInput` (`self.ControlledCopter`) AxisValue))))

(event `InputAction|Toogle Map`
  (params (Key :type "Key Structure"))
  (bind (_screenresolution_x _screenresolution_y) (break `IntPoint` (`self.ScreenResolution`)))
  ;[0.08618 0.3428 1 1 100] Map
  (:`Pressed`
    (`/Engine/EditorBlueprintResources/StandardMacros.FlipFlop`
      (:`A`
        (`self.Possess` (`self.MiniMap`))
        (set `self.bShowMouseCursor` true)
        (`self.SetMouseLocation` (/ _screenresolution_x 2) (/ _screenresolution_y 2))
        (`Widget.SetVisibility` (`self.CopterControllerWidget`) "Collapsed")
        (`Widget.SetVisibility` (`self.MinimapWidget`) "Visible"))
      (:`B`
        (`self.Possess` (`self.ControlledCopter`))
        (set `self.bShowMouseCursor` false)
        (`Widget.SetVisibility` (`self.CopterControllerWidget`) "Visible")
        (`Widget.SetVisibility` (`self.MinimapWidget`) "Collapsed")))))

(event `InputAxis|Copter | Throttle`
  (params (AxisValue :type "Float (single-precision)"))
  ;[0 1 0.3162 1 100] Control
  (`self.SwitchPawns`
    (:`Copter`
      (`Copter.AddCopterThrottleInput` (`self.ControlledCopter`) AxisValue))))

(event `InputAction|Camera | Select`
  (params (Key :type "Key Structure"))
  ;[0.08618 0.3428 1 1 100] Map
  (:`Pressed`
    (`self.SwitchPawns`
      (:`Minimap`
        (`/Game/Copter/Blueprints/Widgets/W_Minimap.StartSelecting` (`self.MinimapWidget`)))))
  (:`Released`
    (`self.SwitchPawns`
      (:`Minimap`
        (`/Game/Copter/Blueprints/Widgets/W_Minimap.StopSelecting` (`self.MinimapWidget`))))))

(event `InputAction|Restart`
  (params (Key :type "Key Structure"))
  ;[0 1 0.3162 1 100] Control
  (:`Pressed`
    (`PrimitiveComponent.SetSimulatePhysics` (`Copter.Mesh` (`self.ControlledCopter`)) false)
    (`Copter.StopFly` (`self.ControlledCopter`))
    (`self.K2_SetActorLocationAndRotation` (`self.ControlledCopter`) (6046.243164 3.556592 120.0) (struct :`Yaw` -180.0) false true)
    (`PrimitiveComponent.SetSimulatePhysics` (`Copter.Mesh` (`self.ControlledCopter`)) true)))

(fn `SmoothAxis`
  (params (AxisValue :type "Float (double-precision)"))
  (returns (Value :type "Float (double-precision)"))
  (locals (Local_PrevAxisValue :type "Float (double-precision)") (Local_PrevDelta :type "Float (double-precision)") (Total_Seconds :type "Float (double-precision)")))

(fn `UpdateWind`
  (bind _outactors (`GameplayStatics.GetAllActorsOfClass` "/Game/Copter/Blueprints/BP_Copter.BP_Copter_C"))
  (for _array_element _outactors
    (bind _output_get (set `self.WindVector` (`KismetMathLibrary.RandomUnitVectorInConeInDegrees` (`self.WindVector`) 50.0)))
    (`PrimitiveComponent.AddForce` (`Copter.Mesh` _array_element) (* _output_get (`self.WindStrength`)) "None" false)))

(fn `UserConstructionScript`)