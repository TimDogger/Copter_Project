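; PID controller Blueprint in the Copter folder that computes an output from input and setpoint.
; Tick accumulates milliseconds to gate Compute to a sample interval; Link sets defaults and tunings.
; Gains are scaled by sample time, with selectable proportional-on-error or on-measurement and a clamped integral sum.
; As wired, InAuto is only ever set false, blocking Compute, whose final clamp forces any non-exceeding output to OutMin.
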(event `self.ReceiveTick`
  (params (DeltaSeconds :type "Float (single-precision)"))
  (set `self.Millis` (+ (`KismetMathLibrary.Round` (* 1000 DeltaSeconds)) (`self.Millis`))))

(fn `Compute`
  (returns (Success :type Boolean))
  (locals (Local_Now :type Integer) (Local_TimeChange :type Integer) (Local_Input :type "Float (double-precision)") (Local_Error :type "Float (double-precision)") (Local_DInput :type "Float (double-precision)"))
  (bind _pid_p (break `/Game/Copter/Structs/K_PID` (`self.PID`)))
  (bind _pid_p_2 (break `/Game/Copter/Structs/K_PID` (`self.PID`)))
  (bind (_pid_p_3 _pid_i) (break `/Game/Copter/Structs/K_PID` (`self.PID`)))
  (bind (_pid_p_4 _pid_i_2 _pid_d) (break `/Game/Copter/Structs/K_PID` (`self.PID`)))
  (if (not (`self.InAuto`))
    (return false)
    (else
      (bind _output_get (set `local.Local_Now` (`self.Millis`)))
      (set `local.Local_TimeChange` (- _output_get (`self.LastTime`)))
      (if (>= (`local.Local_TimeChange`) (`self.SampleTime`))
        (set `local.Local_Error` (- (`self.Setpoint`) (`self.Input`)))
        (set `local.Local_DInput` (- (`local.Local_Input`) (`self.LastInput`)))
        (set `self.OutputSum` (+ (`self.OutputSum`) (* (`local.Local_Error`) _pid_i)))
        (`|ExecutionSequence`
          (:`then_0`
            (if (not (`self.POnE`))
              (set `self.OutputSum` (- (`self.OutputSum`) (* (`local.Local_DInput`) _pid_p)))))
          (:`then_1`
            (if (> (`self.OutputSum`) (`self.OutMax`))
              (set `self.OutputSum` (`self.OutMax`))
              (elif (< (`self.OutputSum`) (`self.OutMin`))
                (set `self.OutputSum` (`self.OutMin`)))))
          (:`then_2`
            (if (`self.POnE`)
              (set `self.Output` (* (`local.Local_Error`) _pid_p_2))
              (else
                (set `self.Output` 0.0))))
          (:`then_3`
            (set `self.Output` (+ (`self.Output`) (- (`self.OutputSum`) (* _pid_d (`local.Local_DInput`)))))
            (if (> (`self.Output`) (`self.OutMax`))
              (set `self.Output` (`self.OutMax`))
              (elif true
                (set `self.Output` (`self.OutMin`)))))
          (:`then_4`
            (set `self.LastInput` (`local.Local_Input`))
            (set `self.LastTime` (`local.Local_Now`))))
        (else
          (return false))))))

(fn `Initialize`
  (set `self.OutputSum` (`self.Output`))
  (set `self.LastInput` (`self.Input`))
  (if (> (`self.OutputSum`) (`self.OutMax`))
    (set `self.OutputSum` (`self.OutMax`))
    (elif (< (`self.OutputSum`) (`self.OutMin`))
      (set `self.OutputSum` (`self.OutMin`)))))

(fn `Link`
  (params (Input :type "Float (double-precision)") (Output :type "Float (double-precision)") (Setpoint :type "Float (double-precision)") (PID :type "/Game/Copter/Structs/K_PID Structure") (POn :type Integer) (ControllerDirection :type Integer))
  (set `self.Input` Input)
  (set `self.Output` Output)
  (set `self.Setpoint` Setpoint)
  (set `self.InAuto` false)
  (`self.SetOutputLimits` 0.0 255.0)
  (set `self.SampleTime` 100)
  (`self.SetControllerDirection` ControllerDirection)
  (`self.SetTunings` PID POn)
  (set `self.LastTime` (- (`self.Millis`) (`self.SampleTime`))))

(fn `SetControllerDirection`
  (params (Direction :type Integer))
  (bind (_pid_p _pid_i _pid_d) (break `/Game/Copter/Structs/K_PID` (`self.PID`)))
  (if (and (`self.InAuto`) (!= Direction (`self.ControllerDirection`)))
    (set `self.PID` (make `/Game/Copter/Structs/K_PID` (- 0.0 _pid_p) (- _pid_i 1.0) (- _pid_d 1.0)))
    (set `self.ControllerDirection` Direction)))

(fn `SetMode`
  (params (Mode :type "/Game/Copter/PID_Controller/PID_Mode Enum" :default "NewEnumerator0"))
  (locals (Local_NewAuto :type Boolean))
  (bind _output_get (set `local.Local_NewAuto` (`|EnumEquality` Mode "NewEnumerator0")))
  (if (and _output_get (`|EnumInequality` (`self.Mode`) "NewEnumerator1"))
    (`self.Initialize`))
  (set `self.InAuto` false))

(fn `SetOutputLimits`
  (params (Min :type "Float (double-precision)") (Max :type "Float (double-precision)"))
  (if (>= Min Max)
    (return)
    (else
      (set `self.OutMin` Min)
      (set `self.OutMax` Max)
      (if (`self.InAuto`)
        (`|ExecutionSequence`
          (:`then_0`
            (if (> (`self.Output`) (`self.OutMax`))
              (set `self.Output` (`self.OutMax`))
              (elif (< (`self.Output`) (`self.OutMin`))
                (set `self.Output` (`self.OutMin`)))))
          (:`then_1`
            (if (> (`self.OutputSum`) (`self.OutMax`))
              (set `self.OutputSum` (`self.OutMax`))
              (elif (< (`self.OutputSum`) (`self.OutMin`))
                (set `self.OutputSum` (`self.OutMin`))))))))))

(fn `SetSampleTime`
  (params (NewSampleTime :type Integer))
  (locals (Local_Ratio :type "Float (double-precision)") (Local_NewSampleTime :type Integer))
  (bind (_pid_p _pid_i _pid_d) (break `/Game/Copter/Structs/K_PID` (`self.PID`)))
  (bind _output_get (set `local.Local_NewSampleTime` NewSampleTime))
  (if (> _output_get 0)
    (set `local.Local_Ratio` (/ (`KismetMathLibrary.Conv_IntToDouble` (`local.Local_NewSampleTime`)) (`KismetMathLibrary.Conv_IntToDouble` (`self.SampleTime`))))
    (set `self.PID` (make `/Game/Copter/Structs/K_PID` _pid_p (* _pid_i (`local.Local_Ratio`)) (/ _pid_d (`local.Local_Ratio`))))
    (set `self.SampleTime` (`local.Local_NewSampleTime`))))

(fn `SetTunings`
  (params (PID :type "/Game/Copter/Structs/K_PID Structure") (POn :type Integer))
  (locals (Local_SampleTimeInSec :type "Float (double-precision)") (Local_InputPID :type "/Game/Copter/Structs/K_PID Structure"))
  (bind (_local_inputpid_p _local_inputpid_i _local_inputpid_d) (break `/Game/Copter/Structs/K_PID` (`local.Local_InputPID`)))
  (bind (_pid_p _pid_i _pid_d) (break `/Game/Copter/Structs/K_PID` (`self.PID`)))
  (bind _output_get (set `local.Local_InputPID` PID))
  (bind (_p _i _d) (break `/Game/Copter/Structs/K_PID` _output_get))
  (if (or (< _p 0.0) (< _i 0.0) (< _d 0.0))
    (return)
    (else
      (bind _output_get_2 (set `self.POn` POn))
      (set `self.POnE` (== _output_get_2 1))
      (set `local.Local_SampleTimeInSec` (`KismetMathLibrary.Conv_IntToDouble` (/ (`self.SampleTime`) 1000)))
      (set `self.PID` (make `/Game/Copter/Structs/K_PID` _local_inputpid_p (* _local_inputpid_i (`local.Local_SampleTimeInSec`)) (/ _local_inputpid_d (`local.Local_SampleTimeInSec`))))
      (if (== (`self.ControllerDirection`) 1)
        (set `self.PID` (make `/Game/Copter/Structs/K_PID` (- 0.0 _pid_p) (- 0.0 _pid_i) (- 0.0 _pid_d)))))))